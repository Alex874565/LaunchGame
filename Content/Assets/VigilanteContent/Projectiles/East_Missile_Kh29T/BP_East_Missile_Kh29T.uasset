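; Visual Blueprint for the East Kh-29T missile projectile, exposing engine effect and fin animation controls.
; On BeginPlay it caches the skeletal mesh's anim instance as its missile-specific Animation Blueprint.
; Eight setter events map normalized inputs to clamped deflection angles for the four front and four rear fins, writing them to that anim instance.
; SetEngineState toggles the thruster effect; no flight or damage logic appears in these graphs.
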(event Custom|SetEngineState
  (params (bEngineActive :type Boolean))
  ;[1 1 1] Set engine state
  (Components|Activation|SetActive (Variables|Default|GetThrusterFX) bEngineActive true))

(event Custom|SetFinFront1Angle
  (params (Angle :type Float%20%28double-precision%29))
  (Variables|/Game/Assets/VigilanteContent/Projectiles/East_Missile_Kh29T/BPA_East_Missile_Kh29T.BPA_East_Missile_Kh29T_C|SetFinFront1Angle (Variables|Default|GetAnimInstance) (Math|Float|MapRangeClamped Angle -1.0 1.0 -45.0 45.0)))

(event Custom|SetFinFront2Angle
  (params (Angle :type Float%20%28double-precision%29))
  (Variables|/Game/Assets/VigilanteContent/Projectiles/East_Missile_Kh29T/BPA_East_Missile_Kh29T.BPA_East_Missile_Kh29T_C|SetFinFront2Angle (Variables|Default|GetAnimInstance) (Math|Float|MapRangeClamped Angle -1.0 1.0 -45.0 45.0)))

(event Custom|SetFinFront3Angle
  (params (Angle :type Float%20%28double-precision%29))
  (Variables|/Game/Assets/VigilanteContent/Projectiles/East_Missile_Kh29T/BPA_East_Missile_Kh29T.BPA_East_Missile_Kh29T_C|SetFinFront3Angle (Variables|Default|GetAnimInstance) (Math|Float|MapRangeClamped Angle -1.0 1.0 -45.0 45.0)))

(event Custom|SetFinFront4Angle
  (params (Angle :type Float%20%28double-precision%29))
  (Variables|/Game/Assets/VigilanteContent/Projectiles/East_Missile_Kh29T/BPA_East_Missile_Kh29T.BPA_East_Missile_Kh29T_C|SetFinFront4Angle (Variables|Default|GetAnimInstance) (Math|Float|MapRangeClamped Angle -1.0 1.0 -45.0 45.0)))

(event Custom|SetFinRear1Angle
  (params (Angle :type Float%20%28double-precision%29))
  (Variables|/Game/Assets/VigilanteContent/Projectiles/East_Missile_Kh29T/BPA_East_Missile_Kh29T.BPA_East_Missile_Kh29T_C|SetFinRear1Angle (Variables|Default|GetAnimInstance) (Math|Float|MapRangeClamped Angle -1.0 1.0 -45.0 45.0)))

(event Custom|SetFinRear2Angle
  (params (Angle :type Float%20%28double-precision%29))
  (Variables|/Game/Assets/VigilanteContent/Projectiles/East_Missile_Kh29T/BPA_East_Missile_Kh29T.BPA_East_Missile_Kh29T_C|SetFinRear2Angle (Variables|Default|GetAnimInstance) (Math|Float|MapRangeClamped Angle -1.0 1.0 -45.0 45.0)))

(event Custom|SetFinRear3Angle
  (params (Angle :type Float%20%28double-precision%29))
  (Variables|/Game/Assets/VigilanteContent/Projectiles/East_Missile_Kh29T/BPA_East_Missile_Kh29T.BPA_East_Missile_Kh29T_C|SetFinRear3Angle (Variables|Default|GetAnimInstance) (Math|Float|MapRangeClamped Angle -1.0 1.0 -45.0 45.0)))

(event Custom|SetFinRear4Angle
  (params (Angle :type Float%20%28double-precision%29))
  (Variables|/Game/Assets/VigilanteContent/Projectiles/East_Missile_Kh29T/BPA_East_Missile_Kh29T.BPA_East_Missile_Kh29T_C|SetFinRear4Angle (Variables|Default|GetAnimInstance) (Math|Float|MapRangeClamped Angle -1.0 1.0 -45.0 45.0)))

(event EventBeginPlay
  (bind _asbpa_east_missile_kh_29t (Utilities|Casting|CastToBPA_East_Missile_Kh29T (Components|SkeletalMesh|GetAnimInstance (Variables|Default|GetSkeletalMesh))))
  (Variables|Default|SetAnimInstance _asbpa_east_missile_kh_29t))

(fn ConstructionScript)