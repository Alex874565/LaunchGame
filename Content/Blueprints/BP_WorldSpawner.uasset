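; BP_WorldSpawner builds an endless vertical level of BP_Platform and BP_Walls actors ahead of the climbing player.
; Tick compares player height to the last spawned heights, then adds a batch of randomly spaced platforms or evenly stacked walls.
; Platform positions are rerolled against MinXYDist from the previous one.
; The X and Y checks are inverted relative to each other: X lands outside that distance, Y within it.
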(event EventBeginPlay
  (Variables|Default|SetLastPlatformZ 1e+01)
  (Variables|Default|SetLastWallZ 1.2e+03))

(event Collision|EventActorBeginOverlap
  (params (OtherActor :type Actor%20Object%20Reference)))

(event EventTick
  (params (DeltaSeconds :type Float%20%28single-precision%29))
  (bind _shouldspawn (CallFunction|ShouldSpawnPlatforms))
  (if _shouldspawn
    (CallFunction|SpawnPlatforms))
  (bind _should_spawn (CallFunction|ShouldSpawnWalls))
  (if _should_spawn
    (CallFunction|SpawnWalls)))

(fn ConstructionScript)

(fn BadPlatformX
  (bind _lastplatformx (Variables|Default|GetLastPlatformX))
  (bind _minxydist (Variables|Default|GetMinXYDist))
  (if (Math|Float|InRange(Float) (Variables|Default|GetNewPlatformX) (- _lastplatformx _minxydist) (+ _lastplatformx _minxydist))
    (return false)
    (else
      (return true))))

(fn FindPlatformX
  (bind _output_get (Variables|Default|SetNewPlatformX (Math|Random|RandomFloatinRange -525.0 525.0) :!label _label))
  (bind _isok (CallFunction|BadPlatformX))
  (while (not _isok)
    (goto _label))
  (Variables|Default|SetLastPlatformX _output_get))

(fn FindPlatformY
  (bind _output_get (Variables|Default|SetNewPlatformY (Math|Random|RandomFloatinRange -525.0 525.0) :!label _label))
  (bind _isok (CallFunction|BadPlatformY))
  (while (not _isok)
    (goto _label))
  (Variables|Default|SetLastPlatformY _output_get))

(fn BadPlatformY
  (bind _lastplatformy (Variables|Default|GetLastPlatformY))
  (bind _minxydist (Variables|Default|GetMinXYDist))
  (if (Math|Float|InRange(Float) (Variables|Default|GetNewPlatformY) (- _lastplatformy _minxydist) (+ _lastplatformy _minxydist))
    (return true)
    (else
      (return false))))

(fn ShouldSpawnPlatforms
  (if (>= (.z (Transformation|GetActorLocation (Game|Player|GetPlayerPawn 0))) (- (Variables|Default|GetLastPlatformZ) 2e+03))
    (return true)
    (else
      (return false))))

(fn SpawnPlatforms
  (bind _output_get (Variables|Default|SetNewPlatformZ (+ 1e+04 (Variables|Default|GetLastPlatformZ))))
  (while (> _output_get (Variables|Default|GetLastPlatformZ))
    (bind _output_get_2 (Variables|Default|SetLastPlatformZ (+ (Math|Random|RandomFloatinRange (Variables|Default|GetMinZDist) (Variables|Default|GetMaxZDist)) (Variables|Default|GetLastPlatformZ))))
    (CallFunction|FindPlatformX)
    (CallFunction|FindPlatformY)
    (Game|SpawnActorfromClass "/Game/Blueprints/BP_Platform.BP_Platform_C" (Math|Transform|MakeTransform (Math|Vector|MakeVector (Variables|Default|GetNewPlatformX) (Variables|Default|GetNewPlatformY) _output_get_2) "0, 0, 0" "1.000000,1.000000,1.000000") "Undefined" "MultiplyWithRoot" 0 0)))

(fn ShouldSpawnWalls
  (if (>= (.z (Transformation|GetActorLocation (Game|Player|GetPlayerPawn 0))) (- (Variables|Default|GetLastWallZ) 2.4e+03))
    (return true)
    (else
      (return false))))

(fn SpawnWalls
  (bind _output_get (Variables|Default|SetNewWallZ (+ 6e+03 (Variables|Default|GetLastWallZ))))
  (while (> _output_get (Variables|Default|GetLastWallZ))
    (bind _output_get_2 (Variables|Default|SetLastWallZ (+ (Variables|Default|GetLastWallZ) 1.2e+03)))
    (Game|SpawnActorfromClass "/Game/Blueprints/BP_Walls.BP_Walls_C" (Math|Transform|MakeTransform (Math|Vector|MakeVector 0.0 0.0 _output_get_2) "0, 0, 0" "1.000000,1.000000,1.000000") "Undefined" "MultiplyWithRoot" 0 0)))