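; BP_Water is a water actor that rises steadily along the world Z axis.
; Tick moves it upward by Speed scaled by delta time, teleport and sweep off, and accumulates TimePassed.
; Speed grows by SpeedIncrease only when TimePassed modulo UpdateTime equals exactly zero, a float comparison that depends on frame timing rather than firing reliably at each interval.
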(event EventBeginPlay)

(event Collision|EventActorBeginOverlap
  (params (OtherActor :type Actor%20Object%20Reference)))

(event EventTick
  (params (DeltaSeconds :type Float%20%28single-precision%29))
  (Transformation|SetActorLocation (+ (Transformation|GetActorLocation) (Math|Vector|MakeVector 0.0 0.0 (* DeltaSeconds (Variables|Default|GetSpeed)))) false false)
  (bind _output_get (Variables|Default|SetTimePassed (+ DeltaSeconds (Variables|Default|GetTimePassed))))
  (if (== (Math|Float|%(Float) _output_get (Variables|Default|GetUpdateTime)) 0.0)
    (Variables|Default|SetSpeed (+ (Variables|Default|GetSpeed) (Variables|Default|GetSpeedIncrease)))))

(fn ConstructionScript)